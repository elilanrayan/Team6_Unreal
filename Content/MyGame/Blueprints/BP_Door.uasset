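; BP_Door is a door actor that slides vertically between its closed position and a raised open position when its Activate event fires.
; BeginPlay caches the start location, and the OpeningDoor timeline lerps the actor from there to a fixed upward offset without sweeping.
; Activate plays the timeline from the start or reverses it from the end based on Closed, which flips only when the timeline finishes.
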(event `self.ReceiveBeginPlay`
  (set `self.StartPoint` (`self.K2_GetActorLocation`)))

(event `/Game/MyGame/Blueprints/Interface/BPI_Activable.Activate`
  (bind _closed (`self.Closed`))
  (bind _startpoint (`self.StartPoint`))
  (if _closed
    (bind (_direction _alpha) (`Timeline|Opening Door` :!via `PlayFromStart` :!label _label)
      (:`Update`
        (`self.K2_SetActorLocation` (`KismetMathLibrary.VLerp` _startpoint (+ _startpoint (0.0 0.0 310.0)) _alpha)))
      (:`Finished`
        (set `self.Closed` (select `bool` _closed :`false` true))))
    (else
      (goto _label :!via `ReverseFromEnd`))))

(fn `UserConstructionScript`)