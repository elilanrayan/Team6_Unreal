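; BP_PaintVerify is an Ink actor that groups overlapping paint collision nodes into connected clusters and reports new links to a paint verify manager.
; While the game instance's DrawCollision flag is on, sphere overlaps merge the other node's neighbor list into its own.
; The merged list is copied to every member, and any member's PaintVerifyManager propagates across the group.
; That manager then receives the new neighbor to verify.
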(event `self.ReceiveBeginPlay`
  (bind _bp_paintcollision (`/Game/MyGame/Blueprints/Interface/BPI_VerifyPaintCollision.TestPaintCollision`))
  (set `self.ListNeighbor` (`|MakeArray` _bp_paintcollision))
  (bind _asgi_name_to_give (cast `/Game/MyGame/Blueprints/GI_Game` (`GameplayStatics.GetGameInstance`)))
  (`/Engine/EditorBlueprintResources/StandardMacros.IsValid` _asgi_name_to_give
    (:`Is Valid`
      (set `self.As GI Name To Give` _asgi_name_to_give))))

(event `self.Sphere.OnComponentBeginOverlap`
  (params (OverlappedComponent :type "PrimitiveComponent Object Reference") (OtherActor :type "Actor Object Reference") (OtherComp :type "PrimitiveComponent Object Reference") (OtherBodyIndex :type Integer) (bFromSweep :type Boolean) (SweepResult :type "HitResult Structure (by ref)"))
  (bind _paintverifymanager (`self.PaintVerifyManager`))
  (if (`/Game/MyGame/Blueprints/GI_Game.DrawCollision` (`self.As GI Name To Give`))
    (bind _bp_paintcollision (message `/Game/MyGame/Blueprints/Interface/BPI_VerifyPaintCollision.TestPaintCollision` OtherActor))
    (`/Engine/EditorBlueprintResources/StandardMacros.IsValid` _bp_paintcollision
      (:`Is Valid`
        (if (not (`KismetArrayLibrary.Array_Contains` (`self.ListNeighbor`) _bp_paintcollision))
          (`KismetArrayLibrary.Array_Append` (`self.ListNeighbor`) (`/Game/MyGame/Blueprints/Ink/BP_PaintVerify.ListNeighbor` _bp_paintcollision))
          (`self.CE_AddToNeighbor` _bp_paintcollision)
          (`/Engine/EditorBlueprintResources/StandardMacros.IsValid` _paintverifymanager
            (:`Is Valid`
              (`/Game/MyGame/Blueprints/Ink/BP_PaintVerifyManager.CE_VerifiyCollider` _paintverifymanager _bp_paintcollision))))))))

(event `CE_AddToNeighbor`
  (params (NewNeighbor :type "/Game/MyGame/Blueprints/Ink/BP_PaintVerify Object Reference"))
  (for _array_element (`self.ListNeighbor`)
    (set `/Game/MyGame/Blueprints/Ink/BP_PaintVerify.ListNeighbor` (`self.ListNeighbor`) _array_element)
    (bind _paintverifymanager (`/Game/MyGame/Blueprints/Ink/BP_PaintVerify.PaintVerifyManager` _array_element))
    (`/Engine/EditorBlueprintResources/StandardMacros.IsValid` _paintverifymanager
      (:`Is Valid`
        (set `self.PaintVerifyManager` _paintverifymanager))))
  (`/Engine/EditorBlueprintResources/StandardMacros.IsValid` (`self.PaintVerifyManager`)
    (:`Is Valid`
      (`self.CE_UpdateManager`))))

(event `CE_UpdateManager`
  (for _array_element (`self.ListNeighbor`)
    (set `/Game/MyGame/Blueprints/Ink/BP_PaintVerify.PaintVerifyManager` (`self.PaintVerifyManager`) _array_element)))

(fn `TestPaintCollision`
  (returns (BP_PaintCollision :type "/Game/MyGame/Blueprints/Ink/BP_PaintVerify Object Reference"))
  (return null))

(fn `UserConstructionScript`)