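; BP_PaintEnd is an Ink actor that acts as an on/off endpoint, relaying its activation state to a linked actor.
; ActualizeState acts only when the incoming state differs from the stored one, sending OnMessage or OffMessage to ActivatedActor.
; On activation it also calls SetLightFunctionMaterial on each linked light; deactivation leaves the lights untouched.
; GetState exposes the current Activated flag.
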(event `/Game/MyGame/Blueprints/Interface/BPI_VerifyPaintCollision.ActualizeState`
  (params (State :type Boolean))
  (bind _activated_actor (`self.Activated Actor`))
  (if (!= State (`self.Activated`))
    (set `self.Activated` (not (`self.Activated`)))
    (if (`self.Activated`)
      (message `/Game/MyGame/Blueprints/Interface/BPI_Activable.On` _activated_actor)
      (for _array_element (`self.Lights`)
        (`LightComponent.SetLightFunctionMaterial` (`Light.LightComponent` _array_element) null))
      (else
        (message `/Game/MyGame/Blueprints/Interface/BPI_Activable.Off` _activated_actor)))))

(fn `GetState`
  (returns (State :type Boolean))
  (return (`self.Activated`)))

(fn `UserConstructionScript`)