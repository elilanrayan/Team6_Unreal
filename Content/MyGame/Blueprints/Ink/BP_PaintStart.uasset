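; BP_PaintStart is a switchable source that sends an on/off state to the paint-collision actors touching it.
; Box overlaps collect actors implementing BPI_VerifyPaintCollision into a neighbor list, activating each new one immediately if the source is on.
; Activate toggles between On and Off, which push the state to every neighbor through ActualizeStateMessage.
; The same loops change the light function material, applying a flicker when off and clearing it when on.
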(event `self.Box.OnComponentBeginOverlap`
  (params (OverlappedComponent :type "PrimitiveComponent Object Reference") (OtherActor :type "Actor Object Reference") (OtherComp :type "PrimitiveComponent Object Reference") (OtherBodyIndex :type Integer) (bFromSweep :type Boolean) (SweepResult :type "HitResult Structure (by ref)"))
  ; Overlap
  (if (`KismetSystemLibrary.DoesImplementInterface` OtherActor "/Game/MyGame/Blueprints/Interface/BPI_VerifyPaintCollision.BPI_VerifyPaintCollision_C")
    (`KismetArrayLibrary.Array_Add` (`self.ListNeighbor`) OtherActor)
    (if (`self.DoActivate`)
      (message `/Game/MyGame/Blueprints/Interface/BPI_VerifyPaintCollision.ActualizeState` OtherActor true))))

(event `/Game/MyGame/Blueprints/Interface/BPI_Activable.Off`
  (set `self.DoActivate` false)
  (for _array_element (`self.ListNeighbor`)
    (message `/Game/MyGame/Blueprints/Interface/BPI_VerifyPaintCollision.ActualizeState` _array_element false)
    (`LightComponent.SetLightFunctionMaterial` (`Light.LightComponent` (`self.Light`)) "/Game/MyGame/Asset/VFX/Lighting/MA_Light_Flicker_02.MA_Light_Flicker_02")))

(event `/Game/MyGame/Blueprints/Interface/BPI_Activable.On`
  (set `self.DoActivate` true)
  (for _array_element (`self.ListNeighbor`)
    (message `/Game/MyGame/Blueprints/Interface/BPI_VerifyPaintCollision.ActualizeState` _array_element true)
    (`LightComponent.SetLightFunctionMaterial` (`Light.LightComponent` (`self.Light`)) null)))

(event `/Game/MyGame/Blueprints/Interface/BPI_Activable.Activate`
  (if (`self.DoActivate`)
    (`/Game/MyGame/Blueprints/Interface/BPI_Activable.Off`)
    (else
      (`self.On`))))

(fn `TestPaintCollision`
  (returns (BP_PaintVerify :type "/Game/MyGame/Blueprints/Ink/BP_PaintVerify Object Reference"))
  (return null))

(fn `UserConstructionScript`)