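; BP_PaintVerifyManager detects when painted ink links its Generator to an End point, then triggers ActivatedActor.
; While the game instance's DrawCollision flag is on, paint colliders overlapping the Generator receive this manager and get verified.
; Colliders without End among their neighbors are told to update, apparently propagating the check along the paint.
; On a match, it clears the flag, waits briefly, destroys every BP_PaintVerify and sends the activate message.
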(event `self.ReceiveBeginPlay`
  (bind _asgi_game (cast `/Game/MyGame/Blueprints/GI_Game` (`GameplayStatics.GetGameInstance`)))
  (`/Engine/EditorBlueprintResources/StandardMacros.IsValid` _asgi_game
    (:`Is Valid`
      (set `self.As GI Name To Give` _asgi_game))))

(event `self.Generator.OnComponentBeginOverlap`
  (params (OverlappedComponent :type "PrimitiveComponent Object Reference") (OtherActor :type "Actor Object Reference") (OtherComp :type "PrimitiveComponent Object Reference") (OtherBodyIndex :type Integer) (bFromSweep :type Boolean) (SweepResult :type "HitResult Structure (by ref)"))
  (if (`/Game/MyGame/Blueprints/GI_Game.DrawCollision` (`self.As GI Name To Give`))
    (bind _bp_paintverify (message `/Game/MyGame/Blueprints/Interface/BPI_VerifyPaintCollision.TestPaintCollision` OtherActor))
    (`/Engine/EditorBlueprintResources/StandardMacros.IsValid` _bp_paintverify
      (:`Is Valid`
        (set `/Game/MyGame/Blueprints/Ink/BP_PaintVerify.PaintVerifyManager` self _bp_paintverify)
        (`self.CE_VerifiyCollider` _bp_paintverify)))))

(event `CE_VerifiyCollider`
  (params (PaintCollider :type "/Game/MyGame/Blueprints/Ink/BP_PaintVerify Object Reference"))
  (`/Engine/EditorBlueprintResources/StandardMacros.IsValid` PaintCollider
    (:`Is Valid`
      (if (`KismetArrayLibrary.Array_Contains` (`/Game/MyGame/Blueprints/Ink/BP_PaintVerify.ListNeighbor` PaintCollider) (`self.End`))
        (set `/Game/MyGame/Blueprints/GI_Game.DrawCollision` false (`self.As GI Name To Give`))
        (`KismetSystemLibrary.PrintString` "detecté")
        (`KismetSystemLibrary.Delay` 0.2)
        (bind _outactors (`GameplayStatics.GetAllActorsOfClass` "/Game/MyGame/Blueprints/Ink/BP_PaintVerify.BP_PaintVerify_C"))
        (bind (_arrayindex _arrayelement) (`/Engine/EditorBlueprintResources/StandardMacros.ReverseForEachLoop` _outactors)
          (:`LoopBody`
            (`self.K2_DestroyActor` _arrayelement))
          (:`Completed`
            (message `/Game/MyGame/Blueprints/Interface/BPI_Activable.Activate` (`self.Activated Actor`))))
        (else
          (set `/Game/MyGame/Blueprints/Ink/BP_PaintVerify.PaintVerifyManager` self PaintCollider)
          (`/Game/MyGame/Blueprints/Ink/BP_PaintVerify.CE_UpdateManager` PaintCollider))))))

(fn `TestPaintCollision`
  (returns (BP_PaintVerify :type "/Game/MyGame/Blueprints/Ink/BP_PaintVerify Object Reference"))
  (return null))

(fn `UserConstructionScript`)