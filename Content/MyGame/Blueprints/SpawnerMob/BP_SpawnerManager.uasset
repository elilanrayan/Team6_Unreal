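; BP_SpawnerManager keeps enemies spawning at random spawners, up to a population cap.
; On BeginPlay it caches all BP_Spawner actors and starts the spawn loop.
; Each pass counts actors implementing BPI_Mob and, if below NbMaxEnemies, calls CESpawn on a random spawner.
; The custom event then waits for the Timer delay and calls itself again, repeating indefinitely.
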(event `self.ReceiveBeginPlay`
  (bind _outactors (`GameplayStatics.GetAllActorsOfClass` "/Game/MyGame/Blueprints/SpawnerMob/BP_Spawner.BP_Spawner_C"))
  (set `self.Spawners` _outactors)
  (`self.CE_SpawnRandom`))

(event `CE_SpawnRandom`
  ; Spawn Random
  (bind _outactors (`GameplayStatics.GetAllActorsWithInterface` "/Game/MyGame/Blueprints/Interface/BPI_Mob.BPI_Mob_C"))
  (if (< (`KismetArrayLibrary.Array_Length` _outactors) (`self.NbMaxEnemies`))
    (`/Game/MyGame/Blueprints/SpawnerMob/BP_Spawner.CE_Spawn` (`KismetArrayLibrary.Array_Random` (`self.Spawners`))))
  (`KismetSystemLibrary.Delay` (`self.Timer`))
  (`self.CE_SpawnRandom`))

(fn `UserConstructionScript`)