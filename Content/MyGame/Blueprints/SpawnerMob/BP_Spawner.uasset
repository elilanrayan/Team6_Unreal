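; BP_Spawner is a mob spawn point that spawns a random mob class only when the player is far enough away.
; The CE_Spawn event compares its distance to player 0 against DistanceFromPlayer, then picks a random entry from Mobs.
; The mob spawns slightly above the spawner, adjusting for collisions and aborting if still blocked.
; Nothing in this Blueprint calls CE_Spawn.
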(event `CE_Spawn`
  ; Spawn
  (if (> (`KismetMathLibrary.Vector_Distance` (`self.K2_GetActorLocation`) (`self.K2_GetActorLocation` (`GameplayStatics.GetPlayerCharacter` 0))) (`self.DistanceFromPlayer`))
    (`|SpawnActorFromClass` (`KismetArrayLibrary.Array_Random` (`self.Mobs`)) (`KismetMathLibrary.MakeTransform` (+ (`self.K2_GetActorLocation`) (0.0 0.0 100.0))) "AdjustIfPossibleButDontSpawnIfColliding" "MultiplyWithRoot" null null)))

(fn `UserConstructionScript`)