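; BP_MusicLevel is a Blueprint that plays level music and pauses it along with the game.
; On BeginPlay it spawns the Music as a 2D sound, stores the audio component and makes itself tickable while paused.
; Tick polls the game's pause state and the component's play state, pausing or unpausing the sound when they disagree and printing a message on each change.
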(event `self.ReceiveBeginPlay`
  (bind _returnvalue (`GameplayStatics.SpawnSound2D` (`self.Music`) 1.0 1.0 0.0 null))
  (set `self.Sound` _returnvalue)
  (`self.SetTickableWhenPaused` true))

(event `self.ReceiveTick`
  (params (DeltaSeconds :type "Float (single-precision)"))
  (bind _returnvalue (select `EAudioComponentPlayState` (`AudioComponent.GetPlayState` (`self.Sound`)) :`Playing` true))
  (if (`GameplayStatics.IsGamePaused`)
    (if _returnvalue
      (`AudioComponent.SetPaused` (`self.Sound`) true)
      (`KismetSystemLibrary.PrintString` "Pause"))
    (elif (not _returnvalue)
      (`AudioComponent.SetPaused` (`self.Sound`) false)
      (`KismetSystemLibrary.PrintString` "Start"))))

(fn `UserConstructionScript`)