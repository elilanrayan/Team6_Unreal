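; Tutorial trigger volume that keeps the player's message ink topped up while they stand inside it.
; Box overlap events track whether the player character is inside.
; Each tick while inside, the player's AmmoMessage is raised to three if it is lower.
; The construction script sizes the box from the InBoxExtent variable.
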(event `self.ReceiveTick`
  (params (DeltaSeconds :type "Float (single-precision)"))
  (bind _returnvalue (`GameplayStatics.GetPlayerCharacter` 0))
  (if (`self.IsPlayerIn`)
    (bind _ammo (message `/Game/MyGame/Blueprints/Interface/BPI_Player.GetAmmo` _returnvalue))
    (if (< _ammo 3)
      (message `/Game/MyGame/Blueprints/Interface/BPI_Player.SetAmmo` _returnvalue 3))))

(event `self.Box.OnComponentBeginOverlap`
  (params (OverlappedComponent :type "PrimitiveComponent Object Reference") (OtherActor :type "Actor Object Reference") (OtherComp :type "PrimitiveComponent Object Reference") (OtherBodyIndex :type Integer) (bFromSweep :type Boolean) (SweepResult :type "HitResult Structure (by ref)"))
  (if (== OtherActor (`GameplayStatics.GetPlayerCharacter` 0))
    (set `self.IsPlayerIn` true)))

(event `self.Box.OnComponentEndOverlap`
  (params (OverlappedComponent :type "PrimitiveComponent Object Reference") (OtherActor :type "Actor Object Reference") (OtherComp :type "PrimitiveComponent Object Reference") (OtherBodyIndex :type Integer))
  (if (== OtherActor (`GameplayStatics.GetPlayerCharacter` 0))
    (set `self.IsPlayerIn` false)))

(fn `UserConstructionScript`
  (`BoxComponent.SetBoxExtent` (`self.Box`) (`self.In Box Extent`) true))