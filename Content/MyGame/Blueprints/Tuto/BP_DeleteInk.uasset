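; BP_DeleteInk is a trigger volume in the Tuto folder that takes away the player's message ammo, apparently their ink.
; When the player character overlaps the box while IsActivable is set and holds message ammo, it zeroes that ammo and destroys itself, so it fires only once.
; An overlap with no ammo leaves the trigger in place.
; The construction script sizes the box from the InBoxExtent variable.
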(event `self.ReceiveBeginPlay`)

(event `self.Box.OnComponentBeginOverlap`
  (params (OverlappedComponent :type "PrimitiveComponent Object Reference") (OtherActor :type "Actor Object Reference") (OtherComp :type "PrimitiveComponent Object Reference") (OtherBodyIndex :type Integer) (bFromSweep :type Boolean) (SweepResult :type "HitResult Structure (by ref)"))
  (bind _returnvalue (`GameplayStatics.GetPlayerCharacter` 0))
  (if (`self.IsActivable`)
    (if (== OtherActor _returnvalue)
      (bind _ammo (message `/Game/MyGame/Blueprints/Interface/BPI_Player.GetAmmo` _returnvalue))
      (if (> _ammo 0)
        (message `/Game/MyGame/Blueprints/Interface/BPI_Player.SetAmmo` _returnvalue 0)
        (set `self.IsActivable` false)
        (`self.K2_DestroyActor`)))))

(fn `UserConstructionScript`
  (`BoxComponent.SetBoxExtent` (`self.Box`) (`self.In Box Extent`) true))