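; BP_CountMob is an actor in the Tuto folder that triggers objects once no BP_Mob actors remain in the world.
; Tick runs through a one-second Delay, throttling a custom event that gathers all BP_Mob actors.
; When that list is empty and CanActivate is true, it clears the flag so activation fires once, then sends ActivateMessage to every entry in ActivableObjects.
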(event `self.ReceiveTick`
  (params (DeltaSeconds :type "Float (single-precision)"))
  (`KismetSystemLibrary.Delay` 1.0)
  (`self.CE_MobEmpty`))

(event `CE_MobEmpty`
  (bind _outactors (`GameplayStatics.GetAllActorsOfClass` "/Game/MyGame/Blueprints/Character/Mobs/BP_Mob.BP_Mob_C"))
  (if (and (`KismetArrayLibrary.Array_IsEmpty` _outactors) (`self.CanActivate`))
    (set `self.CanActivate` false)
    (for _array_element (`self.ActivableObjects`)
      (message `/Game/MyGame/Blueprints/Interface/BPI_Activable.Activate` _array_element))))

(fn `UserConstructionScript`)