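; BP_ShowText is a trigger volume that shows an on-screen text widget, apparently for tutorials, while the player stands inside it.
; Box overlap events filtered to the player character create a new WBP_ShowText and add it to the viewport on entry, then remove it on exit.
; The construction script sizes the box from InBoxExtent; the widget's TXT variable is referenced but unused.
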(event `self.Box.OnComponentBeginOverlap`
  (params (OverlappedComponent :type "PrimitiveComponent Object Reference") (OtherActor :type "Actor Object Reference") (OtherComp :type "PrimitiveComponent Object Reference") (OtherBodyIndex :type Integer) (bFromSweep :type Boolean) (SweepResult :type "HitResult Structure (by ref)"))
  (if (== OtherActor (`GameplayStatics.GetPlayerCharacter` 0))
    (bind _returnvalue (`|CreateWidget` "/Game/UI/WBP_ShowText.WBP_ShowText_C"))
    (bind _output_get (set `self.WBP ShowText` _returnvalue))
    (`UserWidget.AddToViewport` _output_get 0)))

(event `self.Box.OnComponentEndOverlap`
  (params (OverlappedComponent :type "PrimitiveComponent Object Reference") (OtherActor :type "Actor Object Reference") (OtherComp :type "PrimitiveComponent Object Reference") (OtherBodyIndex :type Integer))
  (if (== OtherActor (`GameplayStatics.GetPlayerCharacter` 0))
    (`Widget.RemoveFromParent` (`self.WBP ShowText`))))

(fn `UserConstructionScript`
  (`BoxComponent.SetBoxExtent` (`self.Box`) (`self.In Box Extent`) true))