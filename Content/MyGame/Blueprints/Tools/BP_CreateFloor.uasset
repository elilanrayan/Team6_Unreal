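; BP_CreateFloor is a tool actor that builds a grid of BP_CanvasFloor actors.
; CE_CreateFloor first clears existing floors, then loops over the X and Y of Dimension, spawning tiles spaced by DimensionFloor.
; Each tile attaches to this actor with KeepRelative rules, so the grid offsets become relative to it.
; CE_DeleteAllFloor destroys every BP_CanvasFloor found in the world, not only this actor's tiles.
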(event `CE_DeleteAllFloor`
  (bind _outactors (`GameplayStatics.GetAllActorsOfClass` "/Game/MyGame/Blueprints/Canvas/BP_CanvasFloor.BP_CanvasFloor_C"))
  (bind (_arrayindex _arrayelement) (`/Engine/EditorBlueprintResources/StandardMacros.ReverseForEachLoop` _outactors)
    (:`LoopBody`
      (`self.K2_DestroyActor` _arrayelement))))

(event `CE_CreateFloor`
  (bind (_dimension_x _dimension_y) (`KismetMathLibrary.BreakVector2D` (`self.Dimension`)))
  (bind (_dimensionfloor_x _dimensionfloor_y) (`KismetMathLibrary.BreakVector2D` (`self.DimensionFloor`)))
  (`self.CE_DeleteAllFloor`)
  (for _index (range (+ (`KismetMathLibrary.FTrunc` _dimension_x) 1))
    (for _index_2 (range (+ (`KismetMathLibrary.FTrunc` _dimension_y) 1))
      (bind _returnvalue (`|SpawnActorFromClass` "/Game/MyGame/Blueprints/Canvas/BP_CanvasFloor.BP_CanvasFloor_C" (`KismetMathLibrary.MakeTransform` (`KismetMathLibrary.MakeVector` (* _index _dimensionfloor_x) (* _index_2 _dimensionfloor_y))) "Undefined" "MultiplyWithRoot" null null))
      (`self.K2_AttachToActor` _returnvalue self "None" "KeepRelative" "KeepRelative" "KeepRelative" true))))

(fn `UserConstructionScript`)