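; Light manager that culls the level's Light actors by their distance to the player character.
; BeginPlay caches every Light actor, then starts a custom event that re-calls itself after a one-second delay instead of running on Tick.
; Each pass shows light components closer than DistanceMin and hides those farther away, calling SetVisibility only when the state needs to change.
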(event `self.ReceiveBeginPlay`
  (bind _outactors (`GameplayStatics.GetAllActorsOfClass` "/Script/Engine.Light"))
  (set `self.Lights` _outactors)
  (`self.CE_LightsTest`))

(event `CE_LightsTest`
  (bind _distancemin (`self.DistanceMin`))
  (`KismetSystemLibrary.Delay` 1.0)
  (for _array_element (`self.Lights`)
    (bind _returnvalue (`SceneComponent.IsVisible` (`Light.LightComponent` _array_element)))
    (bind _returnvalue_2 (`KismetMathLibrary.Vector_Distance` (`self.K2_GetActorLocation` _array_element) (`self.K2_GetActorLocation` (`GameplayStatics.GetPlayerCharacter` 0))))
    (if (and (not _returnvalue) (< _returnvalue_2 _distancemin))
      (bind _lightcomponent (`Light.LightComponent` _array_element))
      (`SceneComponent.SetVisibility` _lightcomponent true false)
      (elif (and _returnvalue (> _returnvalue_2 _distancemin))
        (`SceneComponent.SetVisibility` _lightcomponent false false))))
  (`self.CE_LightsTest`))

(fn `UserConstructionScript`)