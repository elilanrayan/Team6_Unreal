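; BP_Item is a pickup actor gated behind a skill check.
; Interact, when allowed, spawns a WBP_SkillCheck widget, cross-links it with the item and first-person character, stuns the player and enables skill check input after a short delay.
; A separate CE_PickUp event marks the player as having the item and destroys the actor after a brief delay.
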(event `self.ReceiveBeginPlay`
  (bind _asbp_first_person_character (cast `/Game/MyGame/Blueprints/Character/BP_FirstPersonCharacter` (`GameplayStatics.GetPlayerCharacter` 0)))
  (set `self.Player` _asbp_first_person_character))

(event `CE_DestroyItem`
  (`KismetSystemLibrary.Delay` 0.2)
  (`self.K2_DestroyActor`))

(event `/Game/MyGame/Blueprints/Interface/BPI_Interact.Interact`
  (bind _player (`self.Player`))
  (if (`self.CanInteract`)
    (bind _returnvalue (`|CreateWidget` "/Game/UI/WBP_SkillCheck.WBP_SkillCheck_C"))
    (bind _output_get (set `self.Skill Check` _returnvalue))
    (set `/Game/MyGame/Blueprints/Character/BP_FirstPersonCharacter.WPB SkillCheck` _output_get (`self.Player`))
    (set `/Game/UI/WBP_SkillCheck.BP Item` self _output_get)
    (`UserWidget.AddToViewport` _output_get 0)
    (set `/Game/MyGame/Blueprints/Character/BP_FirstPersonCharacter.IsStun` true _player)
    (`KismetSystemLibrary.Delay` 0.1)
    (set `/Game/MyGame/Blueprints/Character/BP_FirstPersonCharacter.CanDoSkillCheck` true _player)))

(event `CE_PickUp`
  (set `/Game/MyGame/Blueprints/Character/BP_FirstPersonCharacter.HasItem` true (`self.Player`))
  (`KismetSystemLibrary.PrintString` "PickUp")
  (`self.CE_DestroyItem`))

(fn `UserConstructionScript`)