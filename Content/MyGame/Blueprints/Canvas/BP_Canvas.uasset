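; BP_Canvas is a paintable surface that shows brush strokes on its material through a render target created at BeginPlay.
; Draw stamps a brush material via DrawMaterial and interpolates extra stamps between nearby points to close gaps.
; DrawCollider similarly interpolates world positions, spawning BP_PaintVerify actors where a sphere trace finds none too close.
; A retriggerable delay after Draw resets both stroke histories, separating strokes.
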(event `self.ReceiveBeginPlay`
  (`|ExecutionSequence`
    (:`then_0`
      (bind _returnvalue (`KismetRenderingLibrary.CreateRenderTarget2D` 1024 1024 "RTF_RGBA8_SRGB"))
      (bind _output_get (set `self.RenderTarget` _returnvalue))
      (`KismetRenderingLibrary.ClearRenderTarget2D` _output_get))
    (:`then_1`
      (bind _returnvalue_2 (`KismetMaterialLibrary.CreateDynamicMaterialInstance` (`PrimitiveComponent.GetMaterial` (`self.Object`) 0)))
      (`MaterialInstanceDynamic.SetTextureParameterValue` _returnvalue_2 "RenderTarget" (`self.RenderTarget`))
      (`PrimitiveComponent.SetMaterial` (`self.Object`) 0 _returnvalue_2))
    (:`then_2`
      (bind _returnvalue_3 (`KismetMaterialLibrary.CreateDynamicMaterialInstance` "/Game/Material/Paint/M_Brush.M_Brush"))
      (set `self.BrushMaterial` _returnvalue_3))))

(event `CE_EndDraw`
  (`KismetSystemLibrary.RetriggerableDelay` 0.2)
  (if (not (`KismetMathLibrary.IsZero2D` (`self.LastDraw`)))
    (set `self.LastPos` (0.0 0.0 0.0))
    (set `self.LastDraw` (0.0 0.0))))

(event `/Game/MyGame/Blueprints/Interface/BPI_Draw.Draw`
  (params (DrawLocation :type "Vector2D Structure"))
  (bind _lastdraw (`self.LastDraw`))
  (bind _returnvalue (`KismetMathLibrary.Distance2D` _lastdraw DrawLocation))
  (`self.DrawBrush` (`self.Brush Texture`) DrawLocation (`self.Brush Size`))
  (if (and (not (`KismetMathLibrary.IsZero2D` _lastdraw)) (> _returnvalue 0.01) (< _returnvalue 0.1))
    (for _index (range 1 (+ (`KismetMathLibrary.FTrunc` (/ _returnvalue 0.01)) 1))
      (bind (_returnvalue_x _returnvalue_y) (`KismetMathLibrary.BreakVector` (`KismetMathLibrary.VLerp` (`KismetMathLibrary.Conv_Vector2DToVector` DrawLocation) (`KismetMathLibrary.Conv_Vector2DToVector` (`self.LastDraw`)) (/ (* _index 0.01) _returnvalue))))
      (`self.DrawBrush` (`self.Brush Texture`) (`KismetMathLibrary.MakeVector2D` _returnvalue_x _returnvalue_y) (`self.Brush Size`)))
    (set `self.LastDraw` DrawLocation)
    (`self.CE_EndDraw`)
    (else
      (set `self.LastDraw` DrawLocation)
      (`self.CE_EndDraw`))))

(event `/Game/MyGame/Blueprints/Interface/BPI_Draw.DrawCollider`
  (params (DrawTransform :type "Transform Structure"))
  (bind _location (.location DrawTransform))
  (bind _lastpos (`self.LastPos`))
  (bind _returnvalue (`KismetMathLibrary.Vector_Distance` _lastpos _location))
  (`self.CE_SpawnCollisionDraw` _location)
  (if (and (not (`KismetMathLibrary.Vector_IsZero` _lastpos)) (> _returnvalue 10.0) (< _returnvalue 100.0))
    (for _index (range 1 (+ (`KismetMathLibrary.FTrunc` (/ _returnvalue 12.0)) 1))
      (`self.CE_SpawnCollisionDraw` (`KismetMathLibrary.VLerp` _location (`self.LastPos`) (/ (* _index 12.0) _returnvalue))))
    (set `self.LastPos` _location)
    (else
      (set `self.LastPos` _location))))

(event `CE_SpawnCollisionDraw`
  (params (pos :type "Vector Structure"))
  (bind _outhits (`KismetSystemLibrary.SphereTraceMultiForObjects` pos pos 12.0 (`|MakeArray` "ObjectTypeQuery7" :!type "EObjectTypeQuery Enum")))
  (set `self.CanSpawn` true)
  (for _array_element _outhits
    (if (< (`KismetMathLibrary.Vector_Distance` (`self.K2_GetActorLocation` (`.HitActor` (`GameplayStatics.BreakHitResult` _array_element))) pos) 10.0)
      (set `self.CanSpawn` false)
      (break)))
  (if (`self.CanSpawn`)
    (`|SpawnActorFromClass` "/Game/MyGame/Blueprints/Ink/BP_PaintVerify.BP_PaintVerify_C" (`KismetMathLibrary.MakeTransform` pos) "AlwaysSpawn" "MultiplyWithRoot" null null)))

(fn `DrawBrush`
  (params (BrushTexture :type "Texture2D Object Reference") (DrawLocation :type "Vector2D Structure") (BrushSize :type "Float (double-precision)"))
  (`|ExecutionSequence`
    (:`then_0`
      (`MaterialInstanceDynamic.SetTextureParameterValue` (`self.BrushMaterial`) "BrushTexture" BrushTexture))
    (:`then_1`
      (bind (_canvas _size _context) (`KismetRenderingLibrary.BeginDrawCanvasToRenderTarget` (`self.RenderTarget`)))
      (`Canvas.K2_DrawMaterial` _canvas (`self.BrushMaterial`) (- (* _size DrawLocation) (/ BrushSize 2.0)) (`KismetMathLibrary.Conv_DoubleToVector2D` BrushSize) (0.0 0.0) (1.0 1.0) 0.0 (0.5 0.5))
      (`KismetRenderingLibrary.EndDrawCanvasToRenderTarget` _context))))

(fn `UserConstructionScript`)