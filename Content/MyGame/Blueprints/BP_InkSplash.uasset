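; BP_InkSplash is an ink splash hazard that grows in, lingers, shrinks away and sends a stun message to overlapping actors.
; On BeginPlay, the T_Grow timeline drives actor scale, then after a configurable delay the same timeline plays in reverse.
; The shared Finished pin destroys the actor once scale is near zero.
; Box overlap calls StunMessage on the other actor without filtering.
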(event `self.ReceiveBeginPlay`
  (bind (_direction _grow) (`Timeline|T_Grow` :!via `PlayFromStart` :!label _label)
    (:`Update`
      (`self.SetActorScale3D` _grow))
    (:`Finished`
      (if (== _grow (0.0 0.0 0.0) :`ErrorTolerance` 0.01)
        (`self.K2_DestroyActor`)
        (else
          (`KismetSystemLibrary.Delay` (`self.TimeBeforeDesapearing`))
          (`self.CE_Desapear`))))))

(event `CE_Desapear`
  (goto _label :!via `ReverseFromEnd`))

(event `self.Box.OnComponentBeginOverlap`
  (params (OverlappedComponent :type "PrimitiveComponent Object Reference") (OtherActor :type "Actor Object Reference") (OtherComp :type "PrimitiveComponent Object Reference") (OtherBodyIndex :type Integer) (bFromSweep :type Boolean) (SweepResult :type "HitResult Structure (by ref)"))
  (message `/Game/MyGame/Blueprints/Interface/BPI_Stun.Stun` OtherActor))

(fn `UserConstructionScript`)