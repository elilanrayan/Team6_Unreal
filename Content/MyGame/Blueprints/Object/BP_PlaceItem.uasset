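; Interactable drop spot where the player places a carried message item, marked by a bobbing arrow sprite re-aimed at the player each loop.
; On GameInstance's item-pickup event, it becomes available only if the current enemy state matches its own State.
; An overlap sphere toggles the input widget.
; Interact consumes the player's item, spawns a non-interactable BP_Item, hides the cues and calls an empty follow-up event.
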(event `CE_Anim`
  (bind `_flèche_sprite` (`self.Flèche_Sprite`))
  (bind `_flèche_sprite_2` (`self.Flèche_Sprite`))
  (bind _new_rot (`/Game/BFL/BFL_LookAtPlayer.LookAtPlayer` self))
  (`SceneComponent.K2_SetRelativeRotation` (`self.Flèche_Sprite`) (`KismetMathLibrary.MakeRotator` 0.0 0.0 (+ (.yaw _new_rot) 90.0)) false false)
  (`KismetSystemLibrary.MoveComponentTo` `_flèche_sprite_2` (0.0 0.0 100.0) (`SceneComponent.RelativeRotation` `_flèche_sprite_2`) true true 0.75)
  (`KismetSystemLibrary.MoveComponentTo` `_flèche_sprite` (0.0 0.0 50.0) (`SceneComponent.RelativeRotation` `_flèche_sprite`) true true 0.75)
  (`self.CE_Anim`))

(event `self.ReceiveBeginPlay`
  (bind _asgi_game (cast `/Game/MyGame/Blueprints/GI_Game` (`GameplayStatics.GetGameInstance`)))
  (bind _output_get (set `self.GameInstance` _asgi_game))
  (add `/Game/MyGame/Blueprints/GI_Game.PlayerGetItem` _output_get (delegate `CE_PlayerGetItem`))
  (`self.CE_Anim`))

(event `CE_PlayerGetItem`
  (bind `_flèche_sprite` (`self.Flèche_Sprite`))
  ; GetItem
  (if (== (`/Game/MyGame/Blueprints/GI_Game.CurrentEnemyState` (`self.GameInstance`)) (`self.State`))
    (set `self.CanPlaceItem` true)
    (`PaperSpriteComponent.SetSprite` `_flèche_sprite` "/Game/MyGame/Asset/UI/Arrow/Flèche_Sprite.Flèche_Sprite")
    (else
      (set `self.CanPlaceItem` false)
      (`PaperSpriteComponent.SetSprite` `_flèche_sprite` null))))

(event `/Game/MyGame/Blueprints/Interface/BPI_Interact.Interact`
  (if (`self.CanPlaceItem`)
    (bind _hasitem (message `/Game/MyGame/Blueprints/Interface/BPI_Player.DoHaveItem` (`GameplayStatics.GetPlayerCharacter` 0)))
    (if _hasitem
      (message `/Game/MyGame/Blueprints/Interface/BPI_Player.SetHasItem` (`GameplayStatics.GetPlayerCharacter` 0) false)
      (set `self.CanPlaceItem` false)
      (bind _returnvalue (`|SpawnActorFromClass` "/Game/MyGame/Blueprints/Object/BP_Item.BP_Item_C" (`SceneComponent.K2_GetComponentToWorld` (`self.ItemPosition`)) "AlwaysSpawn" "MultiplyWithRoot" null null))
      (set `/Game/MyGame/Blueprints/Object/BP_Item.CanInteract` false _returnvalue)
      ; On Item
      (add `self.OnDestroyed` _returnvalue (delegate `CE_OnItemDestroy`))
      (`SceneComponent.SetVisibility` (`self.Widget`) false false)
      (`PaperSpriteComponent.SetSprite` (`self.Flèche_Sprite`) null)
      (`self.CE_FollowingInteraction`))))

(event `CE_FollowingInteraction`)

(event `CE_OnItemDestroy` :!signature `self.OnDestroyed`
  (params (DestroyedActor :type "Actor Object Reference"))
  ; On Item
  (set `self.CanPlaceItem` false))

(event `self.SphereInteractDetection.OnComponentBeginOverlap`
  (params (OverlappedComponent :type "PrimitiveComponent Object Reference") (OtherActor :type "Actor Object Reference") (OtherComp :type "PrimitiveComponent Object Reference") (OtherBodyIndex :type Integer) (bFromSweep :type Boolean) (SweepResult :type "HitResult Structure (by ref)"))
  ; Overlap Input Widget
  (if (and (== OtherActor (`GameplayStatics.GetPlayerCharacter` 0)) (`self.CanPlaceItem`))
    (`SceneComponent.SetVisibility` (`self.Widget`) true false)))

(event `self.SphereInteractDetection.OnComponentEndOverlap`
  (params (OverlappedComponent :type "PrimitiveComponent Object Reference") (OtherActor :type "Actor Object Reference") (OtherComp :type "PrimitiveComponent Object Reference") (OtherBodyIndex :type Integer))
  ; Overlap Input Widget
  (if (== OtherActor (`GameplayStatics.GetPlayerCharacter` 0))
    (`SceneComponent.SetVisibility` (`self.Widget`) false false)))

(fn `UserConstructionScript`)