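; BP_LeverDesactivable is a lever, going by its name, whose ability to be interacted with can be switched on and off.
; Activate toggles between the On and Off events based on the CanInteract flag.
; On enables interaction and shows the Widget only if the player character is within 500 units at that moment.
; Off disables interaction and hides the Widget.
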(event `/Game/MyGame/Blueprints/Interface/BPI_Activable.On`
  (set `self.CanInteract` true)
  (if (< (`KismetMathLibrary.Vector_Distance` (`self.K2_GetActorLocation` (`GameplayStatics.GetPlayerCharacter` 0)) (`self.K2_GetActorLocation`)) 500.0)
    (`SceneComponent.SetVisibility` (`self.Widget`) true false)))

(event `/Game/MyGame/Blueprints/Interface/BPI_Activable.Off`
  (set `self.CanInteract` false)
  (`SceneComponent.SetVisibility` (`self.Widget`) false false))

(event `/Game/MyGame/Blueprints/Interface/BPI_Activable.Activate`
  (if (`self.CanInteract`)
    (`/Game/MyGame/Blueprints/Interface/BPI_Activable.Off`)
    (else
      (`self.On`))))

(fn `UserConstructionScript`
  (`parent.UserConstructionScript`))