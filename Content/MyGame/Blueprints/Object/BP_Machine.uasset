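; BP_Machine is an interactive machine that processes pawns behind a moving door and levels up those whose state matches its own.
; An angry enemy entering Box while the machine is idle triggers activation after a short delay and is snapped to Box.
; Activate flip-flops: one call box-traces pawns, respawns them at SpawnPoint, moves BothDoor and levels up matches.
; The next plays a scale animation, then after a delay stops it, returns BothDoor and resets.
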(event `self.Box.OnComponentBeginOverlap`
  (params (OverlappedComponent :type "PrimitiveComponent Object Reference") (OtherActor :type "Actor Object Reference") (OtherComp :type "PrimitiveComponent Object Reference") (OtherBodyIndex :type Integer) (bFromSweep :type Boolean) (SweepResult :type "HitResult Structure (by ref)"))
  (if (and (`KismetSystemLibrary.DoesImplementInterface` OtherActor "/Game/MyGame/Blueprints/Interface/BPI_Enemy.BPI_Enemy_C") (not (`self.Activated`)))
    (if (`BlackboardComponent.GetValueAsBool` (`AIBlueprintHelperLibrary.GetBlackboard` OtherActor) "IsAngry")
      (set `self.Activated` true)
      (`KismetSystemLibrary.Delay` 0.5)
      (message `/Game/MyGame/Blueprints/Interface/BPI_Activable.Activate` self)
      (`self.K2_SetActorLocation` OtherActor (`SceneComponent.K2_GetComponentLocation` (`self.Box`)) false false))))

(event `/Game/MyGame/Blueprints/Interface/BPI_Activable.Activate`
  (bind _returnvalue (`self.K2_GetActorLocation`))
  (bind _bothdoor (`self.BothDoor`))
  (bind _bothdoor_2 (`self.BothDoor`))
  ; Activate
  (`/Engine/EditorBlueprintResources/StandardMacros.FlipFlop`
    (:`A`
      (bind _outhits (`KismetSystemLibrary.BoxTraceMultiForObjects` :`Start` _returnvalue :`End` _returnvalue :`HalfSize` (120.0 120.0 500.0) :`ObjectTypes` (`|MakeArray` "ObjectTypeQuery3" :!type "EObjectTypeQuery Enum") :`DrawDebugType` "ForDuration"))
      (for _array_element _outhits
        (message `/Game/MyGame/Blueprints/Interface/BPI_Player.Respawn` (`.HitActor` (`GameplayStatics.BreakHitResult` _array_element)) (`SceneComponent.K2_GetComponentLocation` (`self.SpawnPoint`))))
      (`KismetSystemLibrary.MoveComponentTo` _bothdoor (0.0 0.0 275.0) (`SceneComponent.RelativeRotation` _bothdoor) true)
      (set `self.Activated` true)
      (for _array_element_2 _outhits
        (bind (_bblockinghit _binitialoverlap _time _distance _location _impactpoint _normal _impactnormal _physmat _hitactor) (`GameplayStatics.BreakHitResult` _array_element_2))
        (bind _level (message `/Game/MyGame/Blueprints/Interface/BPI_Enemy.GetActualState` _hitactor))
        (if (== _level (`self.State`))
          (message `/Game/MyGame/Blueprints/Interface/BPI_Enemy.LevelUp` _hitactor))))
    (:`B`
      (bind (_direction _scale) (`Timeline|Anim` :!via `PlayFromStart` :!label _label)
        (:`Update`
          (`self.SetActorScale3D` _scale)
          (`KismetSystemLibrary.Delay` 10.0)
          (`self.CE_StopAnim`)
          (`KismetSystemLibrary.MoveComponentTo` _bothdoor_2 (0.0 0.0 0.0) (`SceneComponent.RelativeRotation` _bothdoor_2) true true 0.5)
          (set `self.Activated` false))))))

(event `CE_StopAnim`
  ; Activate
  (goto _label :!via `Stop`))

(fn `UserConstructionScript`)