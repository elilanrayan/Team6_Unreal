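; BP_Item is an interactable pickup that the player collects by passing a skill check.
; Interact creates the skill check widget, hands it to the player and stuns them while it runs.
; Success flags the player as holding the item, copies the item's State to the game instance's enemy state, calls its item-pickup event and destroys the item shortly after.
; Destruction removes the widget and clears the stun.
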(event `self.ReceiveBeginPlay`
  (add `self.OnDestroyed` (delegate `ÇE_SkillcheckStop`))
  (bind _asgi_name_to_give (cast `/Game/MyGame/Blueprints/GI_NameToGive` (`GameplayStatics.GetGameInstance`)))
  (set `self.As GI Name To Give` _asgi_name_to_give))

(event `ÇE_SkillcheckStop` :!signature `self.OnDestroyed`
  (params (DestroyedActor :type "Actor Object Reference"))
  (`/Engine/EditorBlueprintResources/StandardMacros.IsValid` (`self.Skill Check`)
    (:`Is Valid`
      (`Widget.RemoveFromParent` (`self.Skill Check`))
      (message `/Game/MyGame/Blueprints/Interface/BPI_Player.SetStun` (`GameplayStatics.GetPlayerCharacter` 0) false))))

(event `CE_DestroyItem`
  (`KismetSystemLibrary.Delay` 0.2)
  (`self.K2_DestroyActor`))

(event `/Game/MyGame/Blueprints/Interface/BPI_Interact.Interact`
  (if (`self.CanInteract`)
    (bind _returnvalue (`|CreateWidget` "/Game/UI/HUD/WBP_SkillCheck.WBP_SkillCheck_C"))
    (bind _output_get (set `self.Skill Check` _returnvalue))
    (message `/Game/MyGame/Blueprints/Interface/BPI_Player.SetSkillCCheck` (`GameplayStatics.GetPlayerCharacter` 0) _output_get)
    (add `/Game/UI/HUD/WBP_SkillCheck.ED_Succes` (`self.Skill Check`) (delegate `CE_PickUp`))
    (`UserWidget.AddToViewport` (`self.Skill Check`) 0)
    (message `/Game/MyGame/Blueprints/Interface/BPI_Player.SetStun` (`GameplayStatics.GetPlayerCharacter` 0) true)))

(event `CE_PickUp`
  (message `/Game/MyGame/Blueprints/Interface/BPI_Player.SetHasItem` (`GameplayStatics.GetPlayerCharacter` 0) true)
  (set `/Game/MyGame/Blueprints/GI_NameToGive.CurrentEnemyState` (`self.State`) (`self.As GI Name To Give`))
  (`/Game/MyGame/Blueprints/GI_NameToGive.PlayerGetItem` (`self.As GI Name To Give`))
  (`KismetSystemLibrary.PrintString` "PickUp")
  (`self.CE_DestroyItem`))

(fn `UserConstructionScript`)