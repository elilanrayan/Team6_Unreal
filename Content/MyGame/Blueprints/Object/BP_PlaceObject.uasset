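; BP_PlaceObject is an interactable spot where the player can put down a carried item.
; It listens to the game instance's PlayerGetItem event and allows placement only when the current enemy state matches its own State.
; Interact checks the player's held-item flag, clears it and spawns a non-interactable BP_Item at ItemPosition.
; A sphere overlap toggles the input prompt widget, showing it only while placement is allowed.
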(event `self.ReceiveBeginPlay`
  (bind _asgi_game (cast `/Game/MyGame/Blueprints/GI_Game` (`GameplayStatics.GetGameInstance`)))
  (bind _output_get (set `self.As GI Name To Give` _asgi_game))
  (add `/Game/MyGame/Blueprints/GI_Game.PlayerGetItem` _output_get (delegate `CE_PlayerGetItem`)))

(event `CE_PlayerGetItem`
  (if (== (`/Game/MyGame/Blueprints/GI_Game.CurrentEnemyState` (`self.As GI Name To Give`)) (`self.State`))
    (set `self.CanPlaceItem` true)
    (else
      (set `self.CanPlaceItem` false))))

(event `/Game/MyGame/Blueprints/Interface/BPI_Interact.Interact`
  (if (`self.CanPlaceItem`)
    (bind _hasitem (message `/Game/MyGame/Blueprints/Interface/BPI_Player.DoHaveItem` (`GameplayStatics.GetPlayerCharacter` 0)))
    (if _hasitem
      (message `/Game/MyGame/Blueprints/Interface/BPI_Player.SetHasItem` (`GameplayStatics.GetPlayerCharacter` 0) false)
      (set `self.CanPlaceItem` false)
      (bind _returnvalue (`|SpawnActorFromClass` "/Game/MyGame/Blueprints/Object/BP_Item.BP_Item_C" (`SceneComponent.K2_GetComponentToWorld` (`self.ItemPosition`)) "AlwaysSpawn" "MultiplyWithRoot" null null))
      (set `/Game/MyGame/Blueprints/Object/BP_Item.CanInteract` false _returnvalue)
      (add `self.OnDestroyed` _returnvalue (delegate `CE_OnItemDestroy`))
      (else
        (`KismetSystemLibrary.PrintString` "pas")))))

(event `CE_OnItemDestroy` :!signature `self.OnDestroyed`
  (params (DestroyedActor :type "Actor Object Reference"))
  (set `self.CanPlaceItem` false))

(event `self.SphereInteractDetection.OnComponentBeginOverlap`
  (params (OverlappedComponent :type "PrimitiveComponent Object Reference") (OtherActor :type "Actor Object Reference") (OtherComp :type "PrimitiveComponent Object Reference") (OtherBodyIndex :type Integer) (bFromSweep :type Boolean) (SweepResult :type "HitResult Structure (by ref)"))
  ; Overlap Input Widget
  (if (and (== OtherActor (`GameplayStatics.GetPlayerCharacter` 0)) (`self.CanPlaceItem`))
    (`SceneComponent.SetVisibility` (`self.Widget`) true false)))

(event `self.SphereInteractDetection.OnComponentEndOverlap`
  (params (OverlappedComponent :type "PrimitiveComponent Object Reference") (OtherActor :type "Actor Object Reference") (OtherComp :type "PrimitiveComponent Object Reference") (OtherBodyIndex :type Integer))
  ; Overlap Input Widget
  (if (== OtherActor (`GameplayStatics.GetPlayerCharacter` 0))
    (`SceneComponent.SetVisibility` (`self.Widget`) false false)))

(fn `UserConstructionScript`)