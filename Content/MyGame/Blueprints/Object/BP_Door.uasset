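; BP_Door is a door actor that slides vertically between its starting position and a raised position each time it is activated.
; Activate checks the Closed flag to play the OpeningDoor timeline forward from the start or in reverse from the end.
; The timeline lerps the actor's location from the point cached at BeginPlay, then flips Closed on finish.
; A door sound plays on activation and stops when movement finishes.
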(event `self.ReceiveBeginPlay`
  (set `self.StartPoint` (`self.K2_GetActorLocation`)))

(event `/Game/MyGame/Blueprints/Interface/BPI_Activable.Activate`
  (if (`self.Closed`)
    (`self.On`)
    (else
      (`self.Off`)))
  (`AudioComponent.Play` (`self.Door_Activate_SFX`) 0.0))

(event `/Game/MyGame/Blueprints/Interface/BPI_Activable.On`
  (bind _startpoint (`self.StartPoint`))
  ; Activate
  (bind (_direction _alpha) (`Timeline|Opening Door` :!via `PlayFromStart` :!label _label)
    (:`Update`
      (`self.K2_SetActorLocation` (`KismetMathLibrary.VLerp` _startpoint (+ _startpoint (0.0 0.0 310.0)) _alpha)))
    (:`Finished`
      (set `self.Closed` (select `bool` (`self.Closed`) :`false` true))
      (`AudioComponent.Stop` (`self.Door_Activate_SFX`)))))

(event `/Game/MyGame/Blueprints/Interface/BPI_Activable.Off`
  ; Activate
  (goto _label :!via `ReverseFromEnd`))

(fn `UserConstructionScript`)