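; BP_Lever is an interactable lever that the player flips between closed and open positions to trigger linked activatable objects.
; Interact locks further input and plays the ShiftLever timeline forward or in reverse, rotating LeverTrack between the two rotations.
; When the timeline finishes, it sends ActivateMessage to each ActivatableRef, then toggles Closed and re-enables interaction after a short delay.
; An overlap volume shows or hides the prompt widget for the player while interaction is allowed.
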(event `/Game/MyGame/Blueprints/Interface/BPI_Interact.Interact`
  ; Interact
  (if (`self.CanInteract`)
    (set `self.CanInteract` false)
    (if (`self.Closed`)
      (bind (_direction _alpha) (`Timeline|ShiftLever` :!via `PlayFromStart` :!label _label)
        (:`Update`
          (`SceneComponent.K2_SetRelativeRotation` (`self.LeverTrack`) (`KismetMathLibrary.RLerp` (`self.ClosedRot`) (`self.OpenRot`) _alpha) false false))
        (:`Finished`
          (for _array_element (`self.Activatable Ref`)
            (message `/Game/MyGame/Blueprints/Interface/BPI_Activable.Activate` _array_element))
          (`KismetSystemLibrary.Delay` 0.2)
          (set `self.CanInteract` true)
          (set `self.Closed` (select `bool` (`self.Closed`) :`false` true))))
      (else
        (goto _label :!via `ReverseFromEnd`)))))

(event `self.InteractDetection.OnComponentBeginOverlap`
  (params (OverlappedComponent :type "PrimitiveComponent Object Reference") (OtherActor :type "Actor Object Reference") (OtherComp :type "PrimitiveComponent Object Reference") (OtherBodyIndex :type Integer) (bFromSweep :type Boolean) (SweepResult :type "HitResult Structure (by ref)"))
  ; Overlap Input Widget
  (if (and (== OtherActor (`GameplayStatics.GetPlayerCharacter` 0)) (`self.CanInteract`))
    (`SceneComponent.SetVisibility` (`self.Widget`) true false)))

(event `self.InteractDetection.OnComponentEndOverlap`
  (params (OverlappedComponent :type "PrimitiveComponent Object Reference") (OtherActor :type "Actor Object Reference") (OtherComp :type "PrimitiveComponent Object Reference") (OtherBodyIndex :type Integer))
  ; Overlap Input Widget
  (if (and (== OtherActor (`GameplayStatics.GetPlayerCharacter` 0)) (`self.CanInteract`))
    (`SceneComponent.SetVisibility` (`self.Widget`) false false)))

(fn `UserConstructionScript`)