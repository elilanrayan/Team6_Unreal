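; BP_Call is a Blueprint in the Phone folder that shows a one-time text message on screen when its CE_Call event fires.
; The event creates a WBP_ShowText widget, passes it the Texts variable and adds it to the viewport.
; A OneShot flag blocks repeat calls, and an optional DoStopPlayer flag calls SetStunMessage on the player character as the message appears.
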(event `CE_Call`
  (if (not (`self.OneShot`))
    (bind _returnvalue (`|CreateWidget` "/Game/UI/WBP_ShowText.WBP_ShowText_C"))
    (bind _output_get (set `self.WBP ShowText` _returnvalue))
    (set `/Game/UI/WBP_ShowText.Texts` (`self.Texts`) _output_get)
    (`UserWidget.AddToViewport` _output_get 0)
    (set `self.OneShot` true)
    (if (`self.DoStopPlayer`)
      (message `/Game/MyGame/Blueprints/Interface/BPI_Player.SetStun` (`GameplayStatics.GetPlayerCharacter` 0) true))))

(fn `UserConstructionScript`)