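; BP_CallByPlace is a placed trigger volume that starts a phone call when the player walks into it.
; It caches GI_Game on BeginPlay and sizes its box from an exposed extent in the construction script.
; On overlap it calls CECall only if the player character has the item message and the game instance's CurrentEnemyState matches the trigger's LevelItem value.
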(event `self.ReceiveBeginPlay`
  (bind _asgi_game (cast `/Game/MyGame/Blueprints/GI_Game` (`GameplayStatics.GetGameInstance`)))
  (set `self.As GI Game` _asgi_game))

(event `self.Box.OnComponentBeginOverlap`
  (params (OverlappedComponent :type "PrimitiveComponent Object Reference") (OtherActor :type "Actor Object Reference") (OtherComp :type "PrimitiveComponent Object Reference") (OtherBodyIndex :type Integer) (bFromSweep :type Boolean) (SweepResult :type "HitResult Structure (by ref)"))
  (bind _returnvalue (`GameplayStatics.GetPlayerCharacter` 0))
  (bind _hasitem (message `/Game/MyGame/Blueprints/Interface/BPI_Player.GetHasItem` _returnvalue))
  (if (and (== OtherActor _returnvalue) _hasitem (== (`/Game/MyGame/Blueprints/GI_Game.CurrentEnemyState` (`self.As GI Game`)) (`self.LevelItem`)))
    (`self.CE_Call`)))

(fn `UserConstructionScript`
  (`BoxComponent.SetBoxExtent` (`self.Box`) (`self.In Box Extent`) true))