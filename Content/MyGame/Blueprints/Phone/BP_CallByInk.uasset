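; Phone call trigger that fires once the first-person character's accumulated lost ammo passes a threshold.
; On BeginPlay it finds the BP_FirstPersonCharacter and binds to its lost-ammo event.
; Each event adds its value to a running count and runs CECall whenever that count exceeds NbFallForText.
; The count is never reset here, so later losses invoke CECall again.
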(event `self.ReceiveBeginPlay`
  (bind _returnvalue (`GameplayStatics.GetActorOfClass` "/Game/MyGame/Blueprints/Character/BP_FirstPersonCharacter.BP_FirstPersonCharacter_C"))
  (add `/Game/MyGame/Blueprints/Character/BP_FirstPersonCharacter.LostAmmoEvent` _returnvalue (delegate `CE_TestCall`)))

(event `CE_TestCall`
  (params (Value :type "Float (double-precision)"))
  (set `self.NbFall` (+ (`self.NbFall`) Value))
  (if (> (`self.NbFall`) (`self.NbFallForText`))
    (`self.CE_Call`)))

(fn `UserConstructionScript`
  (`parent.UserConstructionScript`))