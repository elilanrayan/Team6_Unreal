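; BP_CallByAttack is a phone Blueprint that triggers a call once an enemy has been attacked often enough.
; On BeginPlay it binds to the EDGetAttacked dispatcher of a single BP_Enemy found in the level.
; Each attack increments a counter, and CECall fires on every hit above the NbAttackForText threshold, as the counter never resets.
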(event `self.ReceiveBeginPlay`
  (bind _returnvalue (`GameplayStatics.GetActorOfClass` "/Game/MyGame/Blueprints/Character/BP_Enemy.BP_Enemy_C"))
  (add `/Game/MyGame/Blueprints/Character/BP_Enemy.ED_GetAttacked` _returnvalue (delegate `CE_IsAttacked`)))

(event `CE_IsAttacked`
  (`/Engine/EditorBlueprintResources/StandardMacros.IncrementInt` (`self.NbAttack`)
    (:`  `
      (if (> (`self.NbAttack`) (`self.NbAttackForText`))
        (`self.CE_Call`)))))

(fn `UserConstructionScript`
  (`parent.UserConstructionScript`))