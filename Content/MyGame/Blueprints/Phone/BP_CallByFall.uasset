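; BP_CallByFall is a phone Blueprint that triggers a call once an enemy has fallen more than a set number of times.
; On BeginPlay it binds to the EDFall dispatcher of the first BP_Enemy found in the level.
; Each dispatch increments NbFall, and every one past the NbFallForText threshold runs CECall, with no reset or one-shot guard.
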(event `self.ReceiveBeginPlay`
  (bind _returnvalue (`GameplayStatics.GetActorOfClass` "/Game/MyGame/Blueprints/Character/BP_Enemy.BP_Enemy_C"))
  (add `/Game/MyGame/Blueprints/Character/BP_Enemy.ED_Fall` _returnvalue (delegate `CE_IsAttacked`)))

(event `CE_IsAttacked`
  (`/Engine/EditorBlueprintResources/StandardMacros.IncrementInt` (`self.NbFall`)
    (:`  `
      (if (> (`self.NbFall`) (`self.NbFallForText`))
        (`self.CE_Call`)))))

(fn `UserConstructionScript`
  (`parent.UserConstructionScript`))