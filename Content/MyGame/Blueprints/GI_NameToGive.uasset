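; Game instance Blueprint, judging by its GI_ prefix, holding skeleton save and load events for a single BP_Save slot, "slot1".
; CE_SaveGame creates and writes a new save when none exists, otherwise only loads and casts the existing one.
; CE_LoadGame loads and casts an existing save without using the result.
; Two further SaveGameToSlot calls are unconnected, so existing saves are never rewritten.
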(event `CE_SaveGame`
  ; Save Game
  (bind _returnvalue (`GameplayStatics.DoesSaveGameExist` "slot1"))
  (if _returnvalue
    (bind _returnvalue_2 (`GameplayStatics.LoadGameFromSlot` "slot1"))
    (cast `/Game/MyGame/Blueprints/BP_Save` _returnvalue_2)
    (else
      (bind _returnvalue_3 (`GameplayStatics.CreateSaveGameObject` "/Game/MyGame/Blueprints/BP_Save.BP_Save_C"))
      (`GameplayStatics.SaveGameToSlot` _returnvalue_3 "slot1"))))

(event `CE_LoadGame`
  ; Load Game
  (bind _returnvalue (`GameplayStatics.DoesSaveGameExist` "slot1"))
  (if _returnvalue
    (bind _returnvalue_2 (`GameplayStatics.LoadGameFromSlot` "slot1"))
    (cast `/Game/MyGame/Blueprints/BP_Save` _returnvalue_2)))