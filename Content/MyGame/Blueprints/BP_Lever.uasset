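; BP_Lever is an interactable lever that toggles between closed and open and triggers a linked activatable object.
; Interact plays or reverses the ShiftLever timeline based on the Closed state, lerping LeverTrack's relative rotation between two rotators.
; When the timeline finishes, it sends an Activate message to ActivatableRef, then re-enables interaction and flips Closed after a short delay.
; A CanInteract flag blocks repeated use mid-movement.
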(event `/Game/MyGame/Blueprints/Interface/BPI_Interact.Interact`
  (if (`self.CanInteract`)
    (set `self.CanInteract` false)
    (if (`self.Closed`)
      (bind (_direction _alpha) (`Timeline|ShiftLever` :!via `PlayFromStart` :!label _label)
        (:`Update`
          (`SceneComponent.K2_SetRelativeRotation` (`self.LeverTrack`) (`KismetMathLibrary.RLerp` (`self.ClosedRot`) (`self.OpenRot`) _alpha) false false))
        (:`Finished`
          (message `/Game/MyGame/Blueprints/Interface/BPI_Activable.Activate` (`self.Activatable Ref`))
          (`KismetSystemLibrary.Delay` 0.2)
          (set `self.CanInteract` true)
          (set `self.Closed` (select `bool` (`self.Closed`) :`false` true))))
      (else
        (goto _label :!via `ReverseFromEnd`)))))

(fn `UserConstructionScript`)