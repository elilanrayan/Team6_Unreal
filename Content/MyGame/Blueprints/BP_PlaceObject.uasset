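; BP_PlaceObject is an interactable spot where the first-person player can place a carried item.
; On BeginPlay it caches the BP_FirstPersonCharacter reference.
; On Interact, if still empty, it clears the player's HasItem flag, marks itself filled and spawns a non-interactable BP_Item at the ItemPosition transform.
; An empty-handed interaction with an empty spot only prints a debug string.
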(event `self.ReceiveBeginPlay`
  (bind _asbp_first_person_character (cast `/Game/MyGame/Blueprints/Character/BP_FirstPersonCharacter` (`GameplayStatics.GetPlayerCharacter` 0)))
  (set `self.Player` _asbp_first_person_character))

(event `/Game/MyGame/Blueprints/Interface/BPI_Interact.Interact`
  (if (`self.HisItemPlaced`)
    _
    (elif (`/Game/MyGame/Blueprints/Character/BP_FirstPersonCharacter.HasItem` (`self.Player`))
      (set `/Game/MyGame/Blueprints/Character/BP_FirstPersonCharacter.HasItem` false (`self.Player`))
      (set `self.HisItemPlaced` true)
      (bind _returnvalue (`|SpawnActorFromClass` "/Game/MyGame/Blueprints/BP_Item.BP_Item_C" (`SceneComponent.K2_GetComponentToWorld` (`self.ItemPosition`)) "AlwaysSpawn" "MultiplyWithRoot" null null))
      (set `/Game/MyGame/Blueprints/BP_Item.CanInteract` false _returnvalue)
      (else
        (`KismetSystemLibrary.PrintString` "pas")))))

(fn `UserConstructionScript`)