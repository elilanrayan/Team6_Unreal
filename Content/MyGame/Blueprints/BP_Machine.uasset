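; BP_Machine is an activatable machine with two sliding door components, Porte1 and Porte2.
; When an actor implementing BPI_Stun first overlaps its Box, it latches Activated and sends an Activate message after a short delay.
; The Activate event uses a FlipFlop to quickly slide both doors vertically between an upper and a lower position, alternating on each call.
; Activated is never reset here, so the overlap trigger fires only once.
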(event `self.Box.OnComponentBeginOverlap`
  (params (OverlappedComponent :type "PrimitiveComponent Object Reference") (OtherActor :type "Actor Object Reference") (OtherComp :type "PrimitiveComponent Object Reference") (OtherBodyIndex :type Integer) (bFromSweep :type Boolean) (SweepResult :type "HitResult Structure (by ref)"))
  (if (and (`KismetSystemLibrary.DoesImplementInterface` OtherActor "/Game/MyGame/Blueprints/Interface/BPI_Stun.BPI_Stun_C") (not (`self.Activated`)))
    (set `self.Activated` true)
    (`KismetSystemLibrary.Delay` 0.5)
    (message `/Game/MyGame/Blueprints/Interface/BPI_Activable.Activate` self)))

(event `/Game/MyGame/Blueprints/Interface/BPI_Activable.Activate`
  (bind _porte1 (`self.Porte1`))
  (bind _porte2 (`self.Porte2`))
  (bind _porte1_2 (`self.Porte1`))
  (bind _porte2_2 (`self.Porte2`))
  (`/Engine/EditorBlueprintResources/StandardMacros.FlipFlop`
    (:`A`
      (`KismetSystemLibrary.MoveComponentTo` _porte1_2 (90.0 0.0 10.0) (`SceneComponent.RelativeRotation` _porte1_2) true false 0.1)
      (`KismetSystemLibrary.MoveComponentTo` _porte2_2 (-90.0 0.0 10.0) (`SceneComponent.RelativeRotation` _porte2_2) true false 0.1))
    (:`B`
      (`KismetSystemLibrary.MoveComponentTo` _porte1 (90.0 0.0 -210.0) (`SceneComponent.RelativeRotation` _porte1) true true 0.1)
      (`KismetSystemLibrary.MoveComponentTo` _porte2 (-90.0 0.0 -210.0) (`SceneComponent.RelativeRotation` _porte2) true true 0.1))))

(fn `UserConstructionScript`)