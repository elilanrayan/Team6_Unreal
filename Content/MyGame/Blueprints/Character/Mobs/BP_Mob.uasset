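; BP_Mob is a small enemy mob with a melee attack on the player and an ink-explosion death.
; Attack turns it toward the player and plays the octopus attack montage.
; On the montage notify it plays a random sound and line-traces forward slightly past Distance, damaging a living player through message calls and adding a dirt-camera widget.
; Destroy plays death sound and Niagara effect, then removes the actor.
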(event `/Game/MyGame/Blueprints/Interface/BPI_Mob.Attack`
  (bind _returnvalue (`GameplayStatics.GetPlayerCharacter` 0))
  (bind _returnvalue_2 (`self.K2_GetActorLocation`))
  ; Attack
  (bind _new_rot (`/Game/BFL/BFL_LookAtPlayer.LookAtPlayer` self))
  (`self.K2_SetActorRotation` (`KismetMathLibrary.MakeRotator` 0.0 0.0 (.yaw _new_rot)))
  (`|PlayMontage` (`self.Mesh`) "/Game/Animations/AM_AttackPoulpe.AM_AttackPoulpe" 1.5
    (:`OnNotifyBegin`
      (`GameplayStatics.PlaySoundAtLocation` (`KismetArrayLibrary.Array_Random` (`|MakeArray` "/Game/Sounds/MiniMob/Minimob_Attack_SFX_01.Minimob_Attack_SFX_01" "/Game/Sounds/MiniMob/Minimob_Attack_SFX_02.Minimob_Attack_SFX_02" :!type "SoundBase Object Reference")) _returnvalue_2 (struct) 1.0 1.0 0.0 null null null null)
      (bind _outhit (`KismetSystemLibrary.LineTraceSingleForObjects` _returnvalue_2 (+ (* (`self.GetActorForwardVector`) (+ (`self.Distance`) 50.0)) _returnvalue_2) (`|MakeArray` "ObjectTypeQuery3" :!type "EObjectTypeQuery Enum") false (`|MakeArray` self :!type "Actor Object Reference")))
      (bind (_bblockinghit _binitialoverlap _time _distance _location _impactpoint _normal _impactnormal _physmat _hitactor) (`GameplayStatics.BreakHitResult` _outhit))
      (if (== _hitactor _returnvalue)
        (bind _isalive (message `/Game/MyGame/Blueprints/Interface/BPI_Player.IsAlive` _returnvalue))
        (if _isalive
          (message `/Game/MyGame/Blueprints/Interface/BPI_Player.DoDamage` _hitactor 3.0)
          (bind _returnvalue_3 (`|CreateWidget` "/Game/UI/WBP_DirtCamera.WBP_DirtCamera_C"))
          (`UserWidget.AddToViewport` _returnvalue_3 0))))))

(event `/Game/MyGame/Blueprints/Interface/BPI_Mob.Destroy`
  (bind _returnvalue (`self.K2_GetActorLocation`))
  ; Destroy
  (`GameplayStatics.PlaySoundAtLocation` "/Game/Sounds/MiniMob/Minimob_Death_SFX.Minimob_Death_SFX" _returnvalue (struct) 1.0 1.0 0.0 null null null null)
  (`NiagaraFunctionLibrary.SpawnSystemAtLocation` "/Game/MyGame/Asset/VFX/VFX_Explosion_Poulpe/NS_Explosion_Encre.NS_Explosion_Encre" _returnvalue)
  (`self.K2_DestroyActor`))

(fn `GetDistance`
  (returns (Distance :type "Float (double-precision)"))
  (return (`self.Distance`)))

(fn `UserConstructionScript`)