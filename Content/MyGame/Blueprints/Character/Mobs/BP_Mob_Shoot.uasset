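; BP_Mob_Shoot is a ranged enemy mob, apparently an octopus, that fires projectiles at the player.
; Attack turns it to face the player on yaw only, then plays the shoot montage at increased speed.
; A montage notify spawns BP_MobProjectile at the ShootSpawn transform, syncing the shot with the animation.
; Destroy plays a death sound and a Niagara ink explosion at its location, then removes the actor.
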(event `/Game/MyGame/Blueprints/Interface/BPI_Mob.Attack`
  ; Attack
  (bind _new_rot (`/Game/BFL/BFL_LookAtPlayer.LookAtPlayer` self))
  (`self.K2_SetActorRotation` (`KismetMathLibrary.MakeRotator` 0.0 0.0 (.yaw _new_rot)))
  (`|PlayMontage` (`self.Mesh`) "/Game/Animations/AM_AttackShootPoulpe.AM_AttackShootPoulpe" 1.5
    (:`OnNotifyBegin`
      (`|SpawnActorFromClass` "/Game/MyGame/Blueprints/Character/Mobs/BP_MobProjectile.BP_MobProjectile_C" (`SceneComponent.K2_GetComponentToWorld` (`self.ShootSpawn`)) "AdjustIfPossibleButAlwaysSpawn" "MultiplyWithRoot" null null))))

(event `/Game/MyGame/Blueprints/Interface/BPI_Mob.Destroy`
  (bind _returnvalue (`self.K2_GetActorLocation`))
  ; Destroy
  (`GameplayStatics.PlaySoundAtLocation` "/Game/Sounds/MiniMob/Minimob_Death_SFX.Minimob_Death_SFX" _returnvalue (struct) 1.0 1.0 0.0 null null null null)
  (`NiagaraFunctionLibrary.SpawnSystemAtLocation` "/Game/MyGame/Asset/VFX/VFX_Explosion_Poulpe/NS_Explosion_Encre.NS_Explosion_Encre" _returnvalue)
  (`self.K2_DestroyActor`))

(fn `UserConstructionScript`
  (`parent.UserConstructionScript`))