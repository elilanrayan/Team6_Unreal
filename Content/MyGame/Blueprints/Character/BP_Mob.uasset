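; BP_Mob is an enemy mob that performs a melee attack on the player, using an octopus ("Poulpe") attack montage.
; Attack plays the montage, and its notify fires a short forward line trace against pawns.
; A hit on the player character sends a damage message and adds a dirt-camera widget to the screen.
; A Destroy event removes the actor and prints its name.
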(event `/Game/MyGame/Blueprints/Interface/BPI_Mob.Attack`
  (bind _returnvalue (`self.K2_GetActorLocation`))
  ; Attack
  (`|PlayMontage` (`self.Mesh`) "/Game/Animations/AM_AttackPoulpe.AM_AttackPoulpe" 1.5
    (:`OnNotifyBegin`
      (bind _outhit (`KismetSystemLibrary.LineTraceSingleForObjects` _returnvalue (+ (* (`self.GetActorForwardVector`) 150.0) _returnvalue) (`|MakeArray` "ObjectTypeQuery3" :!type "EObjectTypeQuery Enum") false (`|MakeArray` self :!type "Actor Object Reference") "ForDuration"))
      (bind (_bblockinghit _binitialoverlap _time _distance _location _impactpoint _normal _impactnormal _physmat _hitactor) (`GameplayStatics.BreakHitResult` _outhit))
      (if (== _hitactor (`GameplayStatics.GetPlayerCharacter` 0))
        (message `/Game/MyGame/Blueprints/Interface/BPI_Player.DoDamage` _hitactor 1.0)
        (bind _returnvalue_2 (`|CreateWidget` "/Game/UI/WBP_DirtCamera.WBP_DirtCamera_C"))
        (`UserWidget.AddToViewport` _returnvalue_2 0)))))

(event `/Game/MyGame/Blueprints/Interface/BPI_Mob.Destroy`
  ; Destroy
  (`self.K2_DestroyActor`)
  (`KismetSystemLibrary.PrintString` (`KismetSystemLibrary.GetDisplayName` self)))

(fn `UserConstructionScript`)