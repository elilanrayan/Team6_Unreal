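; Paper2D enemy character that turns to face the player and switches between walk, run and stun states.
; Tick writes whether the player holds the item to the Blackboard and sets IsAngry when true, while Walk and Run set movement speed.
; Flipbooks come from a per-State table, async-loaded in a chain on BeginPlay.
; Stun and WakeUp swap flipbooks and Blackboard flags; waking also destroys the found BP_Item if nearby.
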(event `CE_LoadNewState`
  (bind (_output_walk _output_stun _output_attack) (break `/Game/Data/Strutures/EnemyState` (`|GetArrayItem` (`self.States`) (`self.State`))))
  (`|LoadAsset` _output_walk
    (:`Completed`
      (`|LoadAsset` _output_stun
        (:`Completed`
          (`|LoadAsset` _output_attack))))))

(event `self.ReceiveBeginPlay`
  (`self.CE_LoadNewState`)
  (`/Game/MyGame/Blueprints/Interface/BPI_Mascot.WakeUp`))

(event `self.ReceiveTick`
  (params (DeltaSeconds :type "Float (single-precision)"))
  (`self.CE_LookAtPlayer`)
  (bind _hasitem (message `/Game/MyGame/Blueprints/Interface/BPI_Player.DoHaveItem` (`GameplayStatics.GetPlayerCharacter` 0)))
  (`BlackboardComponent.SetValueAsBool` (`AIBlueprintHelperLibrary.GetBlackboard` null) "IfPlayerAsItem" _hasitem)
  (if _hasitem
    (`BlackboardComponent.SetValueAsBool` (`AIBlueprintHelperLibrary.GetBlackboard` null) "IsAngry" true)))

(event `CE_LookAtPlayer`
  (bind (_returnvalue_roll _returnvalue_pitch _returnvalue_yaw) (`KismetMathLibrary.BreakRotator` (`KismetMathLibrary.FindLookAtRotation` (`self.K2_GetActorLocation`) (`self.K2_GetActorLocation` (`GameplayStatics.GetPlayerCharacter` 0)))))
  (`self.K2_SetActorRotation` (`KismetMathLibrary.MakeRotator` 0.0 0.0 _returnvalue_yaw)))

(event `/Game/MyGame/Blueprints/Interface/BPI_Mascot.Stun`
  (bind (_output_walk _output_stun) (break `/Game/Data/Strutures/EnemyState` (`|GetArrayItem` (`self.States`) (`self.State`))))
  (`SceneComponent.K2_SetRelativeLocation` (`self.PaperFlipbook`) (0.0 0.0 -25.0) false false)
  (`SceneComponent.SetVisibility` (`self.PF_EnemyStun`) true false)
  (`PaperFlipbookComponent.SetLooping` (`self.PaperFlipbook`) false)
  (`PaperFlipbookComponent.SetFlipbook` (`self.PaperFlipbook`) (`|ConvertAsset` _output_stun))
  (`PaperFlipbookComponent.PlayFromStart` (`self.PaperFlipbook`))
  (`BlackboardComponent.SetValueAsBool` (`AIBlueprintHelperLibrary.GetBlackboard` null) "IsStun" true))

(event `/Game/MyGame/Blueprints/Interface/BPI_Mascot.WakeUp`
  (bind _output_walk (break `/Game/Data/Strutures/EnemyState` (`|GetArrayItem` (`self.States`) (`self.State`))))
  (`SceneComponent.K2_SetRelativeLocation` (`self.PaperFlipbook`) (0.0 0.0 0.0) false false)
  (`SceneComponent.SetVisibility` (`self.PF_EnemyStun`) false false)
  (`PaperFlipbookComponent.SetLooping` (`self.PaperFlipbook`) true)
  (`PaperFlipbookComponent.SetFlipbook` (`self.PaperFlipbook`) (`|ConvertAsset` _output_walk))
  (`PaperFlipbookComponent.PlayFromStart` (`self.PaperFlipbook`))
  (`BlackboardComponent.SetValueAsBool` (`AIBlueprintHelperLibrary.GetBlackboard` null) "IsStun" false)
  (`BlackboardComponent.SetValueAsBool` (`AIBlueprintHelperLibrary.GetBlackboard` null) "DropItem" false)
  (`/Game/MyGame/Blueprints/Interface/BPI_Mascot.TakeItemBack`))

(event `/Game/MyGame/Blueprints/Interface/BPI_Mascot.TakeItemBack`
  (bind _returnvalue (`GameplayStatics.GetActorOfClass` "/Game/MyGame/Blueprints/Object/BP_Item.BP_Item_C"))
  (`/Engine/EditorBlueprintResources/StandardMacros.IsValid` _returnvalue
    (:`Is Valid`
      (if (< (`KismetMathLibrary.Vector_Distance` (`self.K2_GetActorLocation` _returnvalue) (`self.K2_GetActorLocation`)) 100.0)
        (`self.K2_DestroyActor` _returnvalue)))))

(event `/Game/MyGame/Blueprints/Interface/BPI_Mascot.Walk`
  (set `CharacterMovementComponent.MaxWalkSpeed` 200.0 (`self.CharacterMovement`)))

(event `/Game/MyGame/Blueprints/Interface/BPI_Mascot.Run`
  (set `CharacterMovementComponent.MaxWalkSpeed` 600.0 (`self.CharacterMovement`)))

(fn `UserConstructionScript`)